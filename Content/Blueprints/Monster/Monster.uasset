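; Monster enemy that moves toward the player on sight and triggers a jump-scare death screen on contact.
; PawnSensing flags the player as seen and issues an AI move to their location at that moment.
; A capsule hit on the player adds the DeathScreen widget each time.
; A DoOnce then plays the scare sound, waits briefly, pauses the game and switches to UI-only input with a cursor.
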(event OnSeePawn(PawnSensing)
  (params (Pawn :type Pawn%20Object%20Reference))
  (bind _asplayer (Utilities|Casting|CastToplayer Pawn))
  (Variables|Default|SetSeenPlayer true)
  (AI|AIMoveTo self (Transformation|GetActorLocation _asplayer) 0 5.0 false))

(event OnComponentHit(CapsuleComponent)
  (params (HitComponent :type Primitive%20Component%20Object%20Reference) (OtherActor :type Actor%20Object%20Reference) (OtherComp :type Primitive%20Component%20Object%20Reference) (NormalImpulse :type Vector :default "0, 0, 0") (Hit :type Hit%20Result%20Structure%20%28by%20ref%29))
  (bind _returnvalue (Game|GetPlayerController 0))
  (bind _asplayer (Utilities|Casting|CastToplayer OtherActor))
  (bind _returnvalue_2 (UserInterface|CreateWidget "/Game/Blueprints/Widgets/DeathScreen.DeathScreen_C"))
  (UserInterface|Viewport|AddtoViewport _returnvalue_2 0)
  (Utilities|FlowControl|DoOnce false
    (:Completed
      (Audio|PlaySoundatLocation "/Game/SoundFX/2021-09-24_-_Jump_Scare_D_-_www_FesliyanStudios_com.2021-09-24_-_Jump_Scare_D_-_www_FesliyanStudios_com" (Transformation|GetActorLocation _asplayer) "0, 0, 0" 1.0 1.0 0.0 0 0 0 0)
      (Utilities|FlowControl|Delay 3.5)
      (Game|SetGamePaused true)
      (Variables|/Script/Engine.PlayerController|SetbShowMouseCursor _returnvalue true)
      (Input|SetInputModeUIOnly _returnvalue 0 "DoNotLock"))))

(event EventBeginPlay
  (AI|AIMoveTo self "0, 0, 0" 0 5.0 false))

(fn ConstructionScript)