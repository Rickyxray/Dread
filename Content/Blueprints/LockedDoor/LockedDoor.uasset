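; LockedDoor is a door actor that the player can open and close with Interact while holding a key.
; Box overlap by the player caches that player, enables input and opens a gate; leaving reverses the input and gate.
; A FlipFlop alternates playing and reversing the OpenCloseDoor timeline, which lerps mesh yaw, with the same sound both ways.
; GetName exposes the door's Name.
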(event OnComponentBeginOverlap(Box)
  (params (OverlappedComponent :type Primitive%20Component%20Object%20Reference) (OtherActor :type Actor%20Object%20Reference) (OtherComp :type Primitive%20Component%20Object%20Reference) (OtherBodyIndex :type Integer) (bFromSweep :type Boolean) (SweepResult :type Hit%20Result%20Structure%20%28by%20ref%29))
  (bind _self self)
  (bind _returnvalue (Transformation|GetActorLocation _self))
  (bind _asplayer (Utilities|Casting|CastToplayer OtherActor))
  (Input|EnableInput (Game|GetPlayerController 0))
  (Utilities|FlowControl|Gate true) ; enters at Open
)

(event OnComponentEndOverlap(Box)
  (params (OverlappedComponent :type Primitive%20Component%20Object%20Reference) (OtherActor :type Actor%20Object%20Reference) (OtherComp :type Primitive%20Component%20Object%20Reference) (OtherBodyIndex :type Integer))
  (bind _self self)
  (bind _returnvalue (Transformation|GetActorLocation _self))
  (Utilities|Casting|CastToplayer OtherActor)
  (Input|DisableInput (Game|GetPlayerController 0))
  (Utilities|FlowControl|Gate true) ; enters at Close
)

(event Input|ActionEvents|InputActionInteract
  (params (Key :type Key%20Structure :default "None"))
  (bind _self self)
  (bind _returnvalue (Transformation|GetActorLocation _self))
  (:Pressed
    (if (Variables|/Game/Blueprints/Player/player.player_C|GetHasKey (stale OnComponentBeginOverlap(Box) _asplayer))
      (Utilities|FlowControl|Gate true
        (:Exit
          (Utilities|FlowControl|FlipFlop
            (:A
              (Audio|PlaySoundatLocation "/Game/SoundFX/door-1-open.door-1-open" _returnvalue "0, 0, 0" 1.0 1.0 0.0 0 0 0 0)
              (bind _door_track (Timeline|Open/Close%20Door Play)
                (:Update
                  (Transformation|SetRelativeRotation (Variables|Default|GetStaticMesh) (Math|Rotator|MakeRotator 0.0 0.0 (Math|Float|Lerp (Variables|Default|GetClosedAngle) (Variables|Default|GetOpenedAngle) _door_track)) false false))))
            (:B
              (Audio|PlaySoundatLocation "/Game/SoundFX/door-1-open.door-1-open" _returnvalue "0, 0, 0" 1.0 1.0 0.0 0 0 0 0)
              (Timeline|Open/Close%20Door Reverse))))))))

(fn ConstructionScript)

(fn GetName
  (return (Variables|Default|GetName)))