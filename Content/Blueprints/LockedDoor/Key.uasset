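; Key pickup actor for the locked door that grants the player a key when interacted with.
; A box overlap caches the overlapping player reference.
; Interact sets that player's HasKey flag, plays an inspect sound at the key's location and destroys the actor.
; Name and Opacity getters expose stored values.
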(event OnComponentBeginOverlap(Box)
  (params (OverlappedComponent :type Primitive%20Component%20Object%20Reference) (OtherActor :type Actor%20Object%20Reference) (OtherComp :type Primitive%20Component%20Object%20Reference) (OtherBodyIndex :type Integer) (bFromSweep :type Boolean) (SweepResult :type Hit%20Result%20Structure%20%28by%20ref%29))
  (bind _asplayer (Utilities|Casting|CastToplayer OtherActor)))

(event EventInteract
  (Variables|/Game/Blueprints/Player/player.player_C|SetHasKey (stale OnComponentBeginOverlap(Box) _asplayer) true)
  (Audio|PlaySoundatLocation "/Game/SoundFX/422709__niamhd00145229__inspect-item.422709__niamhd00145229__inspect-item" (Transformation|GetActorLocation) "0, 0, 0" 1.0 1.0 0.0 0 0 0 0)
  (Actor|DestroyActor))

(fn ConstructionScript)

(fn GetName
  (return (Variables|Default|GetName)))

(fn Opacity
  (return (Variables|Default|GetOpacity_0)))