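; BedHide is an interactable hiding spot that lets the player hide and unhide with the Interact input.
; A box overlap enables the actor's input and opens a gate for that action, closing both when the player leaves.
; Hiding blends the view to this actor and disables player input; unhiding re-enables that input.
; While hidden, a self-calling short-delay loop applies mouse-driven, clamped pitch and yaw to the camera.
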(event OnComponentBeginOverlap(Box)
  (params (OverlappedComponent :type Primitive%20Component%20Object%20Reference) (OtherActor :type Actor%20Object%20Reference) (OtherComp :type Primitive%20Component%20Object%20Reference) (OtherBodyIndex :type Integer) (bFromSweep :type Boolean) (SweepResult :type Hit%20Result%20Structure%20%28by%20ref%29))
  (bind _returnvalue (Game|GetPlayerController 0))
  (bind _asplayer (Utilities|Casting|CastToplayer OtherActor))
  (Variables|Default|SetPlayer%20REF _asplayer)
  (Input|EnableInput (Game|GetPlayerController 0))
  (Utilities|FlowControl|Gate true) ; enters at Open
)

(event OnComponentEndOverlap(Box)
  (params (OverlappedComponent :type Primitive%20Component%20Object%20Reference) (OtherActor :type Actor%20Object%20Reference) (OtherComp :type Primitive%20Component%20Object%20Reference) (OtherBodyIndex :type Integer))
  (bind _returnvalue (Game|GetPlayerController 0))
  (bind _player_ref (Variables|Default|GetPlayer%20REF))
  (Utilities|Casting|CastToplayer OtherActor)
  (Input|DisableInput (Game|GetPlayerController 0))
  (Utilities|FlowControl|Gate true) ; enters at Close
)

(event Custom|MoveCamera
  (if (Variables|/Game/Blueprints/Player/player.player_C|GetIsHiding (Variables|Default|GetPlayer%20REF))
    (Transformation|SetRelativeRotation (Variables|Default|GetCamera) (Math|Rotator|MakeRotator 0.0 (Math|Float|Clamp(Float) (* (stale Input|AxisEvents|InputAxisMouseUp _output_get) -1.0) -1e+01 1e+01) (Math|Float|Clamp(Float) (stale Input|AxisEvents|InputAxisMouseleft _output_get) 6e+01 1.2e+02)) false false)
    (Utilities|FlowControl|Delay 0.001)
    (CallFunction|MoveCamera)))

(event Input|ActionEvents|InputActionInteract
  (params (Key :type Key%20Structure :default "None"))
  (bind _returnvalue (Game|GetPlayerController 0))
  (bind _player_ref (Variables|Default|GetPlayer%20REF))
  (:Pressed
    (Utilities|FlowControl|Gate true :!label _label
      (:Exit
        (if (Variables|/Game/Blueprints/Player/player.player_C|GetIsHiding _player_ref)
          (Default|Un-Hide _player_ref)
          (Input|EnableInput _player_ref _returnvalue)
          (else
            (Default|Hide _player_ref)
            (Utilities|FlowControl|Sequence
              (:then_0
                (Game|Player|SetViewTargetwithBlend _returnvalue self 0.4 "VTBlend_Linear" 0.0 false)
                (CallFunction|MoveCamera)
                (Input|DisableInput _player_ref (Game|GetPlayerController 0)))
              (:then_1
                (Utilities|FlowControl|Delay 0.2)
                (Input|EnableInput (Game|GetPlayerController 0))
                (goto _label Open)))))))))

(event Input|AxisEvents|InputAxisMouseUp
  (params (AxisValue :type Float%20%28single-precision%29))
  (bind _player_ref (Variables|Default|GetPlayer%20REF))
  (if (Variables|/Game/Blueprints/Player/player.player_C|GetIsHiding _player_ref)
    (bind _output_get (Variables|Default|SetPitch (+ (Variables|Default|GetPitch) AxisValue)))
    (else
      (Pawn|Input|AddControllerPitchInput _player_ref AxisValue))))

(event Input|AxisEvents|InputAxisMouseleft
  (params (AxisValue :type Float%20%28single-precision%29))
  (bind _player_ref (Variables|Default|GetPlayer%20REF))
  (if (Variables|/Game/Blueprints/Player/player.player_C|GetIsHiding _player_ref)
    (bind _output_get (Variables|Default|SetYaw (+ (Variables|Default|GetYaw) AxisValue)))
    (else
      (Pawn|Input|AddControllerYawInput _player_ref AxisValue))))

(fn ConstructionScript)